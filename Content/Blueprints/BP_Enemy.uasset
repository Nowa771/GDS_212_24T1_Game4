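; BP_Enemy is a melee enemy that chases player 0 and attacks with a push montage.
; On montage completion, a forward sphere trace damages any pawn hit, then the chase restarts; failed moves do not retry.
; Non-lethal damage launches it backward and upward.
; At zero health it ragdolls its mesh, still issues a random move, and destroys itself after a delay only if that move succeeds; Wonder is an empty event.
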(event Custom|Wonder
  ;[1 1 1] Wonder
)

(event Custom|Chase%20Player
  (bind _attact_trace_pos (Variables|Default|GetAttact%20trace%20Pos))
  (bind _returnvalue (Transformation|GetWorldLocation _attact_trace_pos))
  ;[1 1 1] Chase Player
  (AI|AIMoveTo self "0, 0, 0" (Game|GetPlayerCharacter 0) 5.0 false
    (:OnSuccess
      (Animation|Montage|PlayMontage (Variables|Character|GetMesh) "/Game/Characters/Mannequins/Animations/Manny/Push_Montage.Push_Montage"
        (:OnCompleted
          (bind (_outhit _returnvalue_2) (Collision|SphereTraceForObjects _returnvalue (+ _returnvalue (* (Math|Vector|GetForwardVector _attact_trace_pos) 1e+02)) 2e+01 (Utilities|Array|MakeArray "ObjectTypeQuery3") false 0 "ForDuration"))
          (if _returnvalue_2
            (Game|Damage|ApplyDamage (.HitActor (Collision|BreakHitResult _outhit)) 1e+01 0 0)
            (CallFunction|ChasePlayer)
            (else
              (CallFunction|ChasePlayer))))))))

(event EventBeginPlay
  (CallFunction|ChasePlayer))

(event EventTick
  (params (DeltaSeconds :type Float%20%28single-precision%29))
  ;[1 1 1] Wonder
)

(event Game|Damage|EventAnyDamage
  (params (Damage :type Float%20%28single-precision%29) (DamageType :type Damage%20Type%20Object%20Reference) (InstigatedBy :type Controller%20Object%20Reference) (DamageCauser :type Actor%20Object%20Reference))
  ;[1 1 1] Damage
  (Variables|Default|SetHealth (- (Variables|Default|GetHealth) Damage))
  (if (<= (Variables|Default|GetHealth) 0.0)
    (Physics|SetSimulatePhysics (Variables|Character|GetMesh) true)
    (CallFunction|Wonder)
    ;[1 1 1] Wonder
    (AI|AIMoveTo self (.RandomLocation (AI|Navigation|GetRandomReachablePointinRadius (Transformation|GetActorLocation) 5e+02 0 0)) 0 5.0 false
      (:OnSuccess
        (Utilities|FlowControl|Delay 5.0)
        (Actor|DestroyActor)))
    (else
      (Character|LaunchCharacter (+ (* (Transformation|GetActorForwardVector) -2e+02) (* (Transformation|GetActorUpVector) 2e+02)) false false))))

(fn ConstructionScript)